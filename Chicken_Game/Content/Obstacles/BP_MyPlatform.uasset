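; BP_MyPlatform is a moving platform obstacle that oscillates along the world Y and Z axes.
; Tick accumulates ElapsedTime and feeds it through degree-based cosine and sine, each with its own rate and speed multiplier.
; The result is added as a world offset every frame without sweep or DeltaSeconds scaling, so the travel distance depends on frame rate.
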(event EventBeginPlay)

(event Collision|EventActorBeginOverlap
  (params (OtherActor :type Actor%20Object%20Reference)))

(event EventTick
  (params (DeltaSeconds :type Float%20%28single-precision%29))
  (bind _output_get (Variables|Default|SetElapsedTime (+ DeltaSeconds (Variables|Default|GetElapsedTime))))
  (Transformation|AddActorWorldOffset (Math|Vector|MakeVector 0.0 (* (Math|Trig|Cos(Degrees) (* _output_get (Variables|Default|GetCosRate))) (Variables|Default|GetHSpeed)) (* (Math|Trig|Sin(Degrees) (* _output_get (Variables|Default|GetSinRate))) (Variables|Default|GetVSpeed)))))

(fn ConstructionScript)